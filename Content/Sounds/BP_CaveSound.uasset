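; BP_CaveSound is a placeable sound trigger that plays an ambient cave sound when the archeologist character enters its sphere.
; The construction script applies the cue, attenuation settings and trigger radius from variables to the audio and sphere components.
; An overlap by BP_Archeologist plays the sound from the start; the graph has no logic to stop it on exit.
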(event `self.Sphere Collision.OnComponentBeginOverlap`
  (params (OverlappedComponent :type "PrimitiveComponent Object Reference") (OtherActor :type "Actor Object Reference") (OtherComp :type "PrimitiveComponent Object Reference") (OtherBodyIndex :type Integer) (bFromSweep :type Boolean) (SweepResult :type "HitResult Structure (by ref)"))
  (cast `/Game/Characters/HiddenPerspective/BP_Archeologist` OtherActor)
  (`AudioComponent.Play` (`self.Ambient Sound`) 0.0))

(fn `UserConstructionScript`
  (`AudioComponent.SetSound` (`self.Ambient Sound`) (`self.Cue`))
  (set `AudioComponent.AttenuationSettings` (`self.AmbientSoundAttenuation`) (`self.Ambient Sound`))
  (`SphereComponent.SetSphereRadius` (`self.Sphere Collision`) (`self.SphereRadius`) true))