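; Animation notify that plays a jump sound matched to the surface beneath the animated mesh's owner.
; When triggered, it line-traces 200 units along the owner's negative up vector on the Visibility channel.
; The hit's physical surface type selects a terrain-specific cue, with rock as the fallback.
; Sounds play at the world origin rather than at the owner or hit point.
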(fn `Received_Notify`
  (params (MeshComp :type "SkeletalMeshComponent Object Reference") (Animation :type "AnimSequenceBase Object Reference") (EventReference :type "AnimNotifyEventReference Structure (by ref)"))
  (returns (ReturnValue :type Boolean))
  (bind _returnvalue (`ActorComponent.GetOwner` MeshComp))
  (bind _returnvalue_2 (`Actor.K2_GetActorLocation` _returnvalue))
  ;[1 1 1] Material Detection
  (bind (_outhit _returnvalue_3) (`KismetSystemLibrary.LineTraceSingle` _returnvalue_2 (+ _returnvalue_2 (* (`Actor.GetActorUpVector` _returnvalue) -200.0)) "TraceTypeQuery1"))
  (if _returnvalue_3
    (switch `EPhysicalSurface` (`GameplayStatics.GetSurfaceType` _outhit)
      (:`SurfaceType_Default`
        (`GameplayStatics.PlaySoundAtLocation` "/Game/Sounds/Rock/RockJumpCue.RockJumpCue" (0.0 0.0 0.0) (struct) 1.0 1.0 0.0 null null null null :!label _label))
      (:`SurfaceType1`
        (`GameplayStatics.PlaySoundAtLocation` "/Game/Sounds/Dirt/DirtJumpCue.DirtJumpCue" (0.0 0.0 0.0) (struct) 1.0 1.0 0.0 null null null null))
      (:`SurfaceType2`
        (`GameplayStatics.PlaySoundAtLocation` "/Game/Sounds/Grass/GrassJumpCue.GrassJumpCue" (0.0 0.0 0.0) (struct) 1.0 1.0 0.0 null null null null))
      (:`SurfaceType3`
        (`GameplayStatics.PlaySoundAtLocation` "/Game/Sounds/Gravel/GravelJumpCue.GravelJumpCue" (0.0 0.0 0.0) (struct) 1.0 1.0 0.0 null null null null))
      (:`SurfaceType4`
        (goto _label))
      (:`SurfaceType5`
        (`GameplayStatics.PlaySoundAtLocation` "/Game/Sounds/Snow/SnowJumpCue.SnowJumpCue" (0.0 0.0 0.0) (struct) 1.0 1.0 0.0 null null null null))
      (:`SurfaceType6`
        (`GameplayStatics.PlaySoundAtLocation` "/Game/Sounds/Water/WaterJumpCue.WaterJumpCue" (0.0 0.0 0.0) (struct) 1.0 1.0 0.0 null null null null))
      (:`SurfaceType7`
        (`GameplayStatics.PlaySoundAtLocation` "/Game/Sounds/Wood/WoodJumpCue.WoodJumpCue" (0.0 0.0 0.0) (struct) 1.0 1.0 0.0 null null null null))))
  (return false))