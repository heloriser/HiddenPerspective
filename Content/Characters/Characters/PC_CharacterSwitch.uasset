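; Player controller that lets the player switch possession between the BP_Spirit characters in the level.
; BeginPlay builds the roster from every BP_Spirit actor and records the player character as the current one, provided it is a BP_Spirit.
; The IA_CharacterSwitch input calls NextCharacter, which steps to the following roster entry, wrapping to the first after the last, and possesses it.
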(event `self.ReceiveBeginPlay`
  (bind _outactors (`GameplayStatics.GetAllActorsOfClass` "/Game/Characters/Characters/BP_Spirit.BP_Spirit_C"))
  (set `self.CharacterRoster` _outactors)
  (bind _asbp_spirit (cast `/Game/Characters/Characters/BP_Spirit` (`GameplayStatics.GetPlayerCharacter` 0)))
  (set `self.CurrentCharacter` _asbp_spirit))

(event `EnhancedInput|/Game/Characters/Characters/Input/IA_CharacterSwitch`
  (params (ActionValue :type Boolean) (ElapsedSeconds :type "Float (double-precision)") (TriggeredSeconds :type "Float (double-precision)") (InputAction :type "InputAction Object Reference" :default "/Game/Characters/Characters/Input/IA_CharacterSwitch.IA_CharacterSwitch"))
  (:`Started`
    (`self.NextCharacter`)))

(fn `NextCharacter`
  (locals (Local_Index :type Integer))
  (bind _returnvalue (`KismetArrayLibrary.Array_Find` (`self.CharacterRoster`) (`self.CurrentCharacter`)))
  (bind _returnvalue_2 (+ _returnvalue 1))
  (set `local.Local_Index` _returnvalue)
  (bind _output_get (set `local.Local_Index` (`KismetMathLibrary.SelectInt` _returnvalue_2 0 (`KismetArrayLibrary.Array_IsValidIndex` (`self.CharacterRoster`) _returnvalue_2))))
  (bind _output_get_2 (set `self.CurrentCharacter` (`|GetArrayItem` (`self.CharacterRoster`) _output_get)))
  (`self.Possess` _output_get_2))

(fn `UserConstructionScript`)