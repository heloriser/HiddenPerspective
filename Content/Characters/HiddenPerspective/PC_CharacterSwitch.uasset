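; Player controller that lets the player swap possession between the Archeologist and the Spirit once the Spirit has appeared.
; NextCharacter cycles a two-entry roster; on unpossess, the previous pawn gets a default controller and, if follow is toggled on, chases the active one via re-issued AIMoveTo.
; Tick sets the appearance flag from the first puzzle's checker or immediately in other levels, and caches gamepad axes.
; It also toggles the pause menu.
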(event `self.ReceiveBeginPlay`
  (`KismetSystemLibrary.DelayUntilNextTick`)
  (bind _returnvalue (`GameplayStatics.GetActorOfClass` "/Game/Characters/HiddenPerspective/BP_Spirit.BP_Spirit_C"))
  (`KismetArrayLibrary.Array_Add` (`self.CharacterRoster`) _returnvalue)
  (set `self.OldCharacter` _returnvalue)
  (bind _returnvalue_2 (`GameplayStatics.GetActorOfClass` "/Game/Characters/HiddenPerspective/BP_Archeologist.BP_Archeologist_C"))
  (`KismetArrayLibrary.Array_Add` (`self.CharacterRoster`) _returnvalue_2)
  (bind _asbp_archeologist (cast `/Game/Characters/HiddenPerspective/BP_Archeologist` (`GameplayStatics.GetPlayerCharacter` 0)))
  (set `self.CurrentCharacter` _asbp_archeologist))

(event `EnhancedInput|/Game/Characters/HiddenPerspective/Input/IA_CharacterSwitch`
  (params (ActionValue :type Boolean) (ElapsedSeconds :type "Float (double-precision)") (TriggeredSeconds :type "Float (double-precision)") (InputAction :type "InputAction Object Reference" :default "/Game/Characters/HiddenPerspective/Input/IA_CharacterSwitch.IA_CharacterSwitch"))
  ;[1 1 1] SwitchCharacter
  (:`Started`
    (if (`self.SpiritAppeared`)
      (`/Engine/EditorBlueprintResources/StandardMacros.FlipFlop`
        (:`A`
          (set `self.SpiritCurrent` true))
        (:`B`
          (set `self.SpiritCurrent` false)))
      (`self.NextCharacter`))))

(event `EnhancedInput|/Game/Characters/HiddenPerspective/Input/IA_Pause`
  (params (ActionValue :type Boolean) (ElapsedSeconds :type "Float (double-precision)") (TriggeredSeconds :type "Float (double-precision)") (InputAction :type "InputAction Object Reference" :default "/Game/Characters/HiddenPerspective/Input/IA_Pause.IA_Pause"))
  (bind _returnvalue (`GameplayStatics.GetPlayerController` 0))
  (bind _returnvalue_2 (`GameplayStatics.GetPlayerController` 0))
  ;[1 1 1] PauseMenu
  (:`Started`
    (if (`GameplayStatics.IsGamePaused`)
      (`Widget.RemoveFromParent` (stale _returnvalue_3))
      (`WidgetBlueprintLibrary.SetInputMode_GameOnly` _returnvalue_2)
      (set `PlayerController.bShowMouseCursor` false _returnvalue_2)
      (`GameplayStatics.SetGamePaused` false)
      (else
        (bind _returnvalue_3 (`|CreateWidget` "/Game/UI/WB_InGameMenu.WB_InGameMenu_C"))
        (`UserWidget.AddToViewport` _returnvalue_3 0)
        (`GameplayStatics.SetGamePaused` true)
        (`WidgetBlueprintLibrary.SetInputMode_GameAndUIEx` _returnvalue null)
        (set `PlayerController.bShowMouseCursor` true _returnvalue)))))

(event `self.ReceiveUnPossess`
  (params (UnpossessedPawn :type "Pawn Object Reference"))
  ;[1 1 1] Follow Mechanic
  (if (`self.SpiritAppeared`)
    (`Pawn.SpawnDefaultController` (`self.OldCharacter`))
    (`self.FollowFunction`)))

(event `FollowFunction`
  ;[1 1 1] Follow Mechanic
  (if (`self.SpiritAppeared`)
    (if (`self.Follow`)
      (`|AIMoveTo` (`self.OldCharacter`) (0.0 0.0 0.0) (`self.CurrentCharacter`) 200.0
        (:`OnSuccess`
          (`self.FollowFunction`))))))

(event `EnhancedInput|/Game/Characters/HiddenPerspective/Input/IA_ToggleFollow`
  (params (ActionValue :type Boolean) (ElapsedSeconds :type "Float (double-precision)") (TriggeredSeconds :type "Float (double-precision)") (InputAction :type "InputAction Object Reference" :default "/Game/Characters/HiddenPerspective/Input/IA_ToggleFollow.IA_ToggleFollow"))
  ;[1 1 1] Follow Mechanic
  (:`Started`
    (`/Engine/EditorBlueprintResources/StandardMacros.FlipFlop`
      (:`A`
        (set `self.Follow` true)
        (`self.FollowFunction`))
      (:`B`
        (set `self.Follow` false)
        (`self.FollowFunction`)))))

(event `self.ReceiveTick`
  (params (DeltaSeconds :type "Float (single-precision)"))
  (`KismetSystemLibrary.DelayUntilNextTick`)
  (if (`self.SpiritAppeared`)
    _
    (elif (== (`self.LvlInt`) 0)
      (bind _returnvalue (`GameplayStatics.GetActorOfClass` "/Game/Interactables/RotationCheck/BP_CheckLocationPuzzle1.BP_CheckLocationPuzzle1_C"))
      (set `self.SpiritAppeared` (`/Game/Interactables/RotationCheck/BP_CheckLocationPuzzle1.SpiritAppeared` _returnvalue))
      (else
        (set `self.SpiritAppeared` true))))
  (set `self.GamepadXAxis` (`self.GetInputAxisKeyValue`))
  (set `self.GamepadYAxis` (`self.GetInputAxisKeyValue`)))

(fn `NextCharacter`
  (bind _returnvalue (`KismetArrayLibrary.Array_Find` (`self.CharacterRoster`) (`self.CurrentCharacter`)))
  (bind _returnvalue_2 (+ _returnvalue 1))
  (bind _output_get (set `self.LocalIndex` _returnvalue))
  (set `self.OldCharacter` (`|GetArrayItem` (`self.CharacterRoster`) _output_get))
  (bind _output_get_2 (set `self.LocalIndex` (`KismetMathLibrary.SelectInt` _returnvalue_2 0 (`KismetArrayLibrary.Array_IsValidIndex` (`self.CharacterRoster`) _returnvalue_2))))
  (bind _output_get_3 (set `self.CurrentCharacter` (`|GetArrayItem` (`self.CharacterRoster`) _output_get_2)))
  (`self.Possess` _output_get_3))

(fn `UserConstructionScript`)