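; Rock pressure plate that sinks when overlapped and also acts as a two-plate puzzle checker.
; A timeline lowers Cube1 on overlap and reverses on exit, calling SteppedOn whenever it finishes in either direction.
; FlipFlops toggle two flags from the SteppedOn events of BP_FlowerPressurePlate3 and BP_RockPressurePlate3.
; Tick polls both flags, then moves Cube1 and Cube to a fixed height and marks the puzzle solved.
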(event `self.ReceiveBeginPlay`
  (bind _returnvalue (`GameplayStatics.GetActorOfClass` "/Game/Interactables/PressurePlates/BP_FlowerPressurePlate3.BP_FlowerPressurePlate3_C"))
  (add `/Game/Interactables/PressurePlates/BP_FlowerPressurePlate3.SteppedOn` _returnvalue (delegate `StepedOnFlower`))
  (bind _returnvalue_2 (`GameplayStatics.GetActorOfClass` "/Game/Interactables/PressurePlates/BP_RockPressurePlate3.BP_RockPressurePlate3_C"))
  (add `/Game/Interactables/PressurePlates/BP_RockPressurePlate3.SteppedOn` _returnvalue_2 (delegate `RockStepedOn`)))

(event `StepedOnFlower`
  (`/Engine/EditorBlueprintResources/StandardMacros.FlipFlop`
    (:`A`
      (set `self.StepedOn1` true))
    (:`B`
      (set `self.StepedOn1` false))))

(event `RockStepedOn`
  (`/Engine/EditorBlueprintResources/StandardMacros.FlipFlop`
    (:`A`
      (set `self.StepedOn2` true))
    (:`B`
      (set `self.StepedOn2` false))))

(event `self.ReceiveTick`
  (params (DeltaSeconds :type "Float (single-precision)"))
  (bind _cube1 (`self.Cube1`))
  (bind (_returnvalue_x _returnvalue_y) (`KismetMathLibrary.BreakVector` (`SceneComponent.K2_GetComponentLocation` _cube1)))
  (if (`self.PuzzleSolved`)
    _
    (elif (`self.StepedOn1`)
      (if (`self.StepedOn2`)
        (`SceneComponent.K2_SetWorldLocation` _cube1 (`KismetMathLibrary.MakeVector` _returnvalue_x _returnvalue_y 63188.661084) false false)
        (`SceneComponent.K2_SetWorldLocation` (`self.Cube`) (`KismetMathLibrary.MakeVector` _returnvalue_x _returnvalue_y 63188.661084) false false)
        (set `self.PuzzleSolved` true)))))

(event `self.Box.OnComponentBeginOverlap`
  (params (OverlappedComponent :type "PrimitiveComponent Object Reference") (OtherActor :type "Actor Object Reference") (OtherComp :type "PrimitiveComponent Object Reference") (OtherBodyIndex :type Integer) (bFromSweep :type Boolean) (SweepResult :type "HitResult Structure (by ref)"))
  (bind (_direction _newtrack_0) (`Timeline|StepedOn` :!label _label)
    (:`Update`
      (`SceneComponent.K2_SetRelativeLocation` (`self.Cube1`) (`KismetMathLibrary.MakeVector` -17.0 -4.0 (`KismetMathLibrary.Lerp` 0.0 -7.0 _newtrack_0)) false false))
    (:`Finished`
      (`self.SteppedOn`))))

(event `self.Box.OnComponentEndOverlap`
  (params (OverlappedComponent :type "PrimitiveComponent Object Reference") (OtherActor :type "Actor Object Reference") (OtherComp :type "PrimitiveComponent Object Reference") (OtherBodyIndex :type Integer))
  (goto _label :!via `Reverse`))

(fn `UserConstructionScript`)