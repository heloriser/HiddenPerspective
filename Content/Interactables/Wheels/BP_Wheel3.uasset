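; BP_Wheel3 is an interactable wheel actor that turns in fixed yaw steps and signals the direction of each turn.
; Event1 calls RoLeft and raises the Cube component's relative yaw, while Event2 calls RoRight and lowers it by the same amount.
; Roll and pitch stay unchanged, and the construction script only runs the parent's.
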(event `self.Event1`
  (bind _cube (`self.Cube`))
  (bind (_relativerotation_roll _relativerotation_pitch _relativerotation_yaw) (`KismetMathLibrary.BreakRotator` (`SceneComponent.RelativeRotation` _cube)))
  (`self.RoLeft`)
  (`SceneComponent.K2_SetRelativeRotation` _cube (`KismetMathLibrary.MakeRotator` _relativerotation_roll _relativerotation_pitch (+ _relativerotation_yaw 5.0)) false false))

(event `self.Event2`
  (bind _cube (`self.Cube`))
  (bind (_relativerotation_roll _relativerotation_pitch _relativerotation_yaw) (`KismetMathLibrary.BreakRotator` (`SceneComponent.RelativeRotation` _cube)))
  (`self.RoRight`)
  (`SceneComponent.K2_SetRelativeRotation` _cube (`KismetMathLibrary.MakeRotator` _relativerotation_roll _relativerotation_pitch (- _relativerotation_yaw 5.0)) false false))

(fn `UserConstructionScript`
  (`parent.UserConstructionScript`))