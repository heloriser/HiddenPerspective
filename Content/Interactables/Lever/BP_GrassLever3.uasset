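; BP_GrassLever3 is an interactable lever that stays linked to BP_GrassLever2, moving vertically when that lever is pressed.
; On BeginPlay it binds to that lever's Pressed event, which plays a timeline lerping the world Z of Cube and LeverGroundSmallGrass, both using Cube's X/Y.
; Interaction flip-flops a second timeline that pitches Cube back and forth, calling its own Pressed dispatcher on every update.
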(event `self.ReceiveBeginPlay`
  (bind _returnvalue (`GameplayStatics.GetActorOfClass` "/Game/Interactables/Lever/BP_GrassLever2.BP_GrassLever2_C"))
  (add `/Game/Interactables/Lever/BP_GrassLever2.Pressed` _returnvalue (delegate `Button2Pressed`)))

(event `Button2Pressed`
  (bind _cube (`self.Cube`))
  (bind (_returnvalue_x _returnvalue_y) (`KismetMathLibrary.BreakVector` (`SceneComponent.K2_GetComponentLocation` _cube)))
  (bind (_direction _newtrack_0) (`Timeline|Timeline`)
    (:`Update`
      (`SceneComponent.K2_SetWorldLocation` _cube (`KismetMathLibrary.MakeVector` _returnvalue_x _returnvalue_y (`KismetMathLibrary.Lerp` 72017.943712 72159.248487 _newtrack_0)) false false)
      (`SceneComponent.K2_SetWorldLocation` (`self.Lever_ground_small_grass`) (`KismetMathLibrary.MakeVector` _returnvalue_x _returnvalue_y (`KismetMathLibrary.Lerp` 72017.943712 72159.248487 _newtrack_0)) false false))))

(event `self.BeginInteraction`
  (`parent.BeginInteraction`)
  (`/Engine/EditorBlueprintResources/StandardMacros.FlipFlop`
    (:`A`
      (bind (_direction _newtrack_0) (`Timeline|Lever` :!label _label)
        (:`Update`
          (`SceneComponent.K2_SetRelativeRotation` (`self.Cube`) (`KismetMathLibrary.MakeRotator` 0.0 (`KismetMathLibrary.Lerp` -20.0 20.0 _newtrack_0)) false false)
          (`self.Pressed`))))
    (:`B`
      (goto _label :!via `Reverse`))))

(fn `UserConstructionScript`
  (`parent.UserConstructionScript`))