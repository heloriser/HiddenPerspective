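; Third Spirit Grass lever: an interactable that moves vertically when BP_SpiritGrassLever2 is pressed and tilts when used.
; On BeginPlay it binds to that lever's Pressed event, which plays a timeline setting Cube and Cube1 between hard-coded world Z heights at Cube's X/Y.
; Interaction flip-flops a second timeline forward and back to pitch Cube1, firing its own Pressed on every timeline update rather than once.
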(event `self.ReceiveBeginPlay`
  (bind _returnvalue (`GameplayStatics.GetActorOfClass` "/Game/Interactables/Lever/BP_SpiritGrassLever2.BP_SpiritGrassLever2_C"))
  (add `/Game/Interactables/Lever/BP_SpiritGrassLever2.Pressed` _returnvalue (delegate `Button2Pressed`)))

(event `Button2Pressed`
  (bind _cube (`self.Cube`))
  (bind (_returnvalue_x _returnvalue_y) (`KismetMathLibrary.BreakVector` (`SceneComponent.K2_GetComponentLocation` _cube)))
  (bind (_direction _newtrack_0) (`Timeline|Timeline_0`)
    (:`Update`
      (`SceneComponent.K2_SetWorldLocation` _cube (`KismetMathLibrary.MakeVector` _returnvalue_x _returnvalue_y (`KismetMathLibrary.Lerp` 62553.173706 62781.308914 _newtrack_0)) false false)
      (`SceneComponent.K2_SetWorldLocation` (`self.Cube1`) (`KismetMathLibrary.MakeVector` _returnvalue_x _returnvalue_y (`KismetMathLibrary.Lerp` 62553.173706 62781.308914 _newtrack_0)) false false))))

(event `self.BeginInteraction`
  (`parent.BeginInteraction`)
  (`/Engine/EditorBlueprintResources/StandardMacros.FlipFlop`
    (:`A`
      (bind (_direction _newtrack_0) (`Timeline|Timeline` :!label _label)
        (:`Update`
          (`SceneComponent.K2_SetRelativeRotation` (`self.Cube1`) (`KismetMathLibrary.MakeRotator` 0.0 (`KismetMathLibrary.Lerp` -20.0 20.0 _newtrack_0)) false false)
          (`self.Pressed`))))
    (:`B`
      (goto _label :!via `Reverse`))))

(fn `UserConstructionScript`
  (`parent.UserConstructionScript`))