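; Second grass lever interactable, which moves vertically into place when BP_GrassLever1 fires its Pressed event.
; On BeginPlay it binds to that lever, and the event plays a timeline lerping the ground grass mesh and Cube between hard-coded world heights, using Cube's X and Y for both.
; Interaction flip-flops the Lever timeline forward and back to pitch the Cube, broadcasting its own Pressed event on every timeline update.
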(event `self.ReceiveBeginPlay`
  (bind _returnvalue (`GameplayStatics.GetActorOfClass` "/Game/Interactables/Lever/BP_GrassLever1.BP_GrassLever1_C"))
  (add `/Game/Interactables/Lever/BP_GrassLever1.Pressed` _returnvalue (delegate `Button2Pressed`)))

(event `Button2Pressed`
  (bind (_returnvalue_x _returnvalue_y) (`KismetMathLibrary.BreakVector` (`SceneComponent.K2_GetComponentLocation` (`self.Cube`))))
  (bind (_direction _newtrack_0) (`Timeline|Timeline`)
    (:`Update`
      (`SceneComponent.K2_SetWorldLocation` (`self.Lever_ground_small_grass`) (`KismetMathLibrary.MakeVector` _returnvalue_x _returnvalue_y (`KismetMathLibrary.Lerp` 72488.27927 72705.743628 _newtrack_0)) false false)
      (`SceneComponent.K2_SetWorldLocation` (`self.Cube`) (`KismetMathLibrary.MakeVector` _returnvalue_x _returnvalue_y (`KismetMathLibrary.Lerp` 72488.27927 72705.743628 _newtrack_0)) false false))))

(event `self.BeginInteraction`
  (`parent.BeginInteraction`)
  (`/Engine/EditorBlueprintResources/StandardMacros.FlipFlop`
    (:`A`
      (bind (_direction _newtrack_0) (`Timeline|Lever` :!label _label)
        (:`Update`
          (`SceneComponent.K2_SetRelativeRotation` (`self.Cube`) (`KismetMathLibrary.MakeRotator` 0.0 (`KismetMathLibrary.Lerp` -20.0 20.0 _newtrack_0)) false false)
          (`self.Pressed`))))
    (:`B`
      (goto _label :!via `Reverse`))))

(fn `UserConstructionScript`
  (`parent.UserConstructionScript`))