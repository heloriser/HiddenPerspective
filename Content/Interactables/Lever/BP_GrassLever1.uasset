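; Grass-covered lever that becomes raised into view by brushing and can then be toggled through player interaction.
; At BeginPlay it binds to the first found BP_BrushInteractable's Brushed event, which plays a timeline lerping the lever and grass between hard-coded world heights.
; Interaction, gated by IsBrushed, flip-flops a second timeline that pitches the lever forward or back, calling Pressed on every update tick.
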(event `self.ReceiveBeginPlay`
  (bind _returnvalue (`GameplayStatics.GetActorOfClass` "/Game/Interactables/Item_Interactions/Brush_Interactables/BP_BrushInteractable.BP_BrushInteractable_C"))
  (add `/Game/Interactables/Item_Interactions/Brush_Interactables/BP_BrushInteractable.Brushed` _returnvalue (delegate `Brushed`)))

(event `Brushed`
  (bind _cube (`self.Cube`))
  (bind (_returnvalue_x _returnvalue_y) (`KismetMathLibrary.BreakVector` (`SceneComponent.K2_GetComponentLocation` _cube)))
  (bind (_direction _newtrack_0) (`Timeline|Timeline`)
    (:`Update`
      (`SceneComponent.K2_SetWorldLocation` _cube (`KismetMathLibrary.MakeVector` _returnvalue_x _returnvalue_y (`KismetMathLibrary.Lerp` 73157.446525 73326.805286 _newtrack_0)) false false)
      (`SceneComponent.K2_SetWorldLocation` (`self.Lever_ground_small_grass`) (`KismetMathLibrary.MakeVector` _returnvalue_x _returnvalue_y (`KismetMathLibrary.Lerp` 73157.446525 73326.805286 _newtrack_0)) false false))))

(event `self.BeginInteraction`
  (`parent.BeginInteraction`)
  (if (`self.IsBrushed`)
    (`/Engine/EditorBlueprintResources/StandardMacros.FlipFlop`
      (:`A`
        (bind (_direction _newtrack_0) (`Timeline|Lever` :!label _label)
          (:`Update`
            (`SceneComponent.K2_SetRelativeRotation` (`self.Cube`) (`KismetMathLibrary.MakeRotator` 0.0 (`KismetMathLibrary.Lerp` -20.0 20.0 _newtrack_0)) false false)
            (`self.Pressed`))))
      (:`B`
        (goto _label :!via `Reverse`)))))

(fn `UserConstructionScript`
  (`parent.UserConstructionScript`))