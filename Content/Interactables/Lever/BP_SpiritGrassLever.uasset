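; Interactable lever that only responds to interaction once IsShoveld is true.
; Each accepted interaction flip-flops a timeline between play and reverse, tilting Cube1 in pitch between two opposite angles.
; The Spirit1Pressed dispatcher is called on every timeline update, so it fires repeatedly during movement in both directions.
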(event `self.BeginInteraction`
  (`parent.BeginInteraction`)
  (if (`self.IsShoveld`)
    (`/Engine/EditorBlueprintResources/StandardMacros.FlipFlop`
      (:`A`
        (bind (_direction _newtrack_0) (`Timeline|Timeline` :!label _label)
          (:`Update`
            (`SceneComponent.K2_SetRelativeRotation` (`self.Cube1`) (`KismetMathLibrary.MakeRotator` 0.0 (`KismetMathLibrary.Lerp` -20.0 20.0 _newtrack_0)) false false)
            (`self.Spirit1Pressed`))))
      (:`B`
        (goto _label :!via `Reverse`)))))

(fn `UserConstructionScript`
  (`parent.UserConstructionScript`))