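; BP_SpiritGrassLever1 is an interactable lever that also rises when another lever, BP_GrassLever3, is pressed.
; On BeginPlay it binds to that lever's Pressed event, which plays a timeline lerping Cube and Cube1 between hardcoded world heights at Cube's X/Y.
; Interaction flip-flops a second timeline forward and back to pitch Cube1, broadcasting its own Pressed on every timeline update rather than once.
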(event `self.ReceiveBeginPlay`
  (bind _returnvalue (`GameplayStatics.GetActorOfClass` "/Game/Interactables/Lever/BP_GrassLever3.BP_GrassLever3_C"))
  (add `/Game/Interactables/Lever/BP_GrassLever3.Pressed` _returnvalue (delegate `Button2Pressed`)))

(event `Button2Pressed`
  (bind _cube (`self.Cube`))
  (bind (_returnvalue_x _returnvalue_y) (`KismetMathLibrary.BreakVector` (`SceneComponent.K2_GetComponentLocation` _cube)))
  (bind (_direction _newtrack_0) (`Timeline|Timeline_0`)
    (:`Update`
      (`SceneComponent.K2_SetWorldLocation` _cube (`KismetMathLibrary.MakeVector` _returnvalue_x _returnvalue_y (`KismetMathLibrary.Lerp` 71176.070932 71352.802908 _newtrack_0)) false false)
      (`SceneComponent.K2_SetWorldLocation` (`self.Cube1`) (`KismetMathLibrary.MakeVector` _returnvalue_x _returnvalue_y (`KismetMathLibrary.Lerp` 71176.070932 71352.802908 _newtrack_0)) false false))))

(event `self.BeginInteraction`
  (`parent.BeginInteraction`)
  (`/Engine/EditorBlueprintResources/StandardMacros.FlipFlop`
    (:`A`
      (bind (_direction _newtrack_0) (`Timeline|Timeline` :!label _label)
        (:`Update`
          (`SceneComponent.K2_SetRelativeRotation` (`self.Cube1`) (`KismetMathLibrary.MakeRotator` 0.0 (`KismetMathLibrary.Lerp` -20.0 20.0 _newtrack_0)) false false)
          (`self.Pressed`))))
    (:`B`
      (goto _label :!via `Reverse`))))

(fn `UserConstructionScript`
  (`parent.UserConstructionScript`))