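; BP_CheckLocationPuzzle3 checks the player's position and facing to complete a three-part visibility puzzle.
; On BeginPlay it binds to three pressure plates: two permanently reveal their meshes, while the third toggles its mesh with a FlipFlop.
; Tick waits until something overlaps the Box, all three meshes are visible and BP_Archeologist's yaw nears a target angle.
; It then, once only, marks the puzzle solved, destroys the three mesh actors and calls Done.
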(event `self.ReceiveBeginPlay`
  (`KismetSystemLibrary.DelayUntilNextTick`)
  (bind _returnvalue (`GameplayStatics.GetActorOfClass` "/Game/Interactables/PressurePlates/BP_PressurePlate.BP_PressurePlate_C"))
  (add `/Game/Interactables/PressurePlates/BP_PressurePlate.MakeVisibale` _returnvalue (delegate `CustomEvent`))
  (bind _returnvalue_2 (`GameplayStatics.GetActorOfClass` "/Game/Interactables/PressurePlates/BP_PressurePlate1.BP_PressurePlate1_C"))
  (add `/Game/Interactables/PressurePlates/BP_PressurePlate1.MakeVisibale` _returnvalue_2 (delegate `MakeVisibale2`))
  (bind _returnvalue_3 (`GameplayStatics.GetActorOfClass` "/Game/Interactables/PressurePlates/BP_PressurePlate2.BP_PressurePlate2_C"))
  (add `/Game/Interactables/PressurePlates/BP_PressurePlate2.MakeVisibale` _returnvalue_3 (delegate `CustomEvent_1`)))

(event `CustomEvent`
  (bind _returnvalue (`GameplayStatics.GetActorOfClass` "/Game/Interactables/PressurePlates/ReatToPressurePlate/PlaneCutOtherPart3_Blueprint.PlaneCutOtherPart3_Blueprint_C"))
  (`SceneComponent.SetVisibility` (`StaticMeshActor.StaticMeshComponent` _returnvalue) true false)
  (set `self.Visibale1` true))

(event `MakeVisibale2`
  (bind _returnvalue (`GameplayStatics.GetActorOfClass` "/Game/Interactables/PressurePlates/ReatToPressurePlate/PlaneCutOtherPart4_Blueprint.PlaneCutOtherPart4_Blueprint_C"))
  (`SceneComponent.SetVisibility` (`StaticMeshActor.StaticMeshComponent` _returnvalue) true false)
  (set `self.Visibale2` true))

(event `CustomEvent_1`
  (if (not (`self.PuzzleSolved`))
    (bind _returnvalue (`GameplayStatics.GetActorOfClass` "/Game/Interactables/PressurePlates/ReatToPressurePlate/Box15_Blueprint1.Box15_Blueprint1_C"))
    (`/Engine/EditorBlueprintResources/StandardMacros.FlipFlop`
      (:`A`
        (bind _staticmeshcomponent (`StaticMeshActor.StaticMeshComponent` _returnvalue))
        (`SceneComponent.SetVisibility` _staticmeshcomponent true false)
        (set `self.Visibale3` true))
      (:`B`
        (`SceneComponent.SetVisibility` _staticmeshcomponent false false)
        (set `self.Visibale3` false)))))

(event `self.ReceiveTick`
  (params (DeltaSeconds :type "Float (single-precision)"))
  (if (`self.ColissionP3`)
    (if (`self.Visibale1`)
      (if (`self.Visibale2`)
        (if (`self.Visibale3`)
          (bind _returnvalue (`GameplayStatics.GetActorOfClass` "/Game/Characters/HiddenPerspective/BP_Archeologist.BP_Archeologist_C"))
          (bind (_returnvalue_roll _returnvalue_pitch _returnvalue_yaw) (`KismetMathLibrary.BreakRotator` (`self.K2_GetActorRotation` _returnvalue)))
          (if (`KismetMathLibrary.NearlyEqual_FloatFloat` _returnvalue_yaw -110.0 20.0)
            (`/Engine/EditorBlueprintResources/StandardMacros.DoOnce` false
              (:`Completed`
                (set `self.PuzzleSolved` true)
                (bind _returnvalue_2 (`GameplayStatics.GetActorOfClass` "/Game/Interactables/PressurePlates/ReatToPressurePlate/PlaneCutOtherPart3_Blueprint.PlaneCutOtherPart3_Blueprint_C"))
                (`self.K2_DestroyActor` _returnvalue_2)
                (bind _returnvalue_3 (`GameplayStatics.GetActorOfClass` "/Game/Interactables/PressurePlates/ReatToPressurePlate/PlaneCutOtherPart4_Blueprint.PlaneCutOtherPart4_Blueprint_C"))
                (`self.K2_DestroyActor` _returnvalue_3)
                (bind _returnvalue_4 (`GameplayStatics.GetActorOfClass` "/Game/Interactables/PressurePlates/ReatToPressurePlate/Box15_Blueprint1.Box15_Blueprint1_C"))
                (`self.K2_DestroyActor` _returnvalue_4)
                (`self.Done`)))))))))

(event `self.Box.OnComponentBeginOverlap`
  (params (OverlappedComponent :type "PrimitiveComponent Object Reference") (OtherActor :type "Actor Object Reference") (OtherComp :type "PrimitiveComponent Object Reference") (OtherBodyIndex :type Integer) (bFromSweep :type Boolean) (SweepResult :type "HitResult Structure (by ref)"))
  (set `self.ColissionP3` true))

(event `self.Box.OnComponentEndOverlap`
  (params (OverlappedComponent :type "PrimitiveComponent Object Reference") (OtherActor :type "Actor Object Reference") (OtherComp :type "PrimitiveComponent Object Reference") (OtherBodyIndex :type Integer))
  (set `self.ColissionP3` false))

(fn `UserConstructionScript`)