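; BP_CheckLocation is a trigger that checks whether BP_Archeologist faces a set direction while its box is overlapped.
; Box begin and end overlap events toggle a collision flag without filtering which actor overlaps.
; While the flag is set, Tick looks up the archeologist by class and runs CallTest every frame its yaw is within a tolerance of 90 degrees.
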(event `self.ReceiveTick`
  (params (DeltaSeconds :type "Float (single-precision)"))
  (if (`self.Colission`)
    (bind _returnvalue (`GameplayStatics.GetActorOfClass` "/Game/Characters/HiddenPerspective/BP_Archeologist.BP_Archeologist_C"))
    (bind (_returnvalue_roll _returnvalue_pitch _returnvalue_yaw) (`KismetMathLibrary.BreakRotator` (`self.K2_GetActorRotation` _returnvalue)))
    (if (`KismetMathLibrary.NearlyEqual_FloatFloat` _returnvalue_yaw 90.0 10.0)
      (`self.Test`))))

(event `self.Box.OnComponentBeginOverlap`
  (params (OverlappedComponent :type "PrimitiveComponent Object Reference") (OtherActor :type "Actor Object Reference") (OtherComp :type "PrimitiveComponent Object Reference") (OtherBodyIndex :type Integer) (bFromSweep :type Boolean) (SweepResult :type "HitResult Structure (by ref)"))
  (set `self.Colission` true))

(event `self.Box.OnComponentEndOverlap`
  (params (OverlappedComponent :type "PrimitiveComponent Object Reference") (OtherActor :type "Actor Object Reference") (OtherComp :type "PrimitiveComponent Object Reference") (OtherBodyIndex :type Integer))
  (set `self.Colission` false))

(fn `UserConstructionScript`)