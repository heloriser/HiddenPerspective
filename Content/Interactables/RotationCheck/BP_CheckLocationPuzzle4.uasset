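; BP_CheckLocationPuzzle4 is a trigger that checks whether the archeologist stands in the right place, facing the right way, to solve a puzzle.
; Box overlaps from any actor set a collision flag.
; Until solved, Tick polls that flag, the visibility flags on two puzzle-piece actors, and BP_Archeologist's yaw against a target within a tolerance.
; On success it destroys three puzzle actors once and calls the Done dispatcher.
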(event `self.ReceiveTick`
  (params (DeltaSeconds :type "Float (single-precision)"))
  (if (not (`self.PuzzleSolved`))
    (`KismetSystemLibrary.DelayUntilNextTick`)
    (bind _returnvalue (`GameplayStatics.GetActorOfClass` "/Game/Interactables/Item_Interactions/Brush_Interactables/PlaneCutOtherPart25_Blueprint.PlaneCutOtherPart25_Blueprint_C"))
    (set `self.Visibale1` (`/Game/Interactables/Item_Interactions/Brush_Interactables/PlaneCutOtherPart25_Blueprint.Visibale` _returnvalue))
    (bind _returnvalue_2 (`GameplayStatics.GetActorOfClass` "/Game/Interactables/Item_Interactions/Brush_Interactables/Box25_Blueprint.Box25_Blueprint_C"))
    (set `self.Visibale2` (`/Game/Interactables/Item_Interactions/Brush_Interactables/Box25_Blueprint.Visibale` _returnvalue_2))
    (if (`self.Visibale1`)
      (if (`self.Visibale2`)
        (if (`self.ColissionP3`)
          (bind _returnvalue_3 (`GameplayStatics.GetActorOfClass` "/Game/Characters/HiddenPerspective/BP_Archeologist.BP_Archeologist_C"))
          (bind (_returnvalue_roll _returnvalue_pitch _returnvalue_yaw) (`KismetMathLibrary.BreakRotator` (`self.K2_GetActorRotation` _returnvalue_3)))
          (if (`KismetMathLibrary.NearlyEqual_FloatFloat` _returnvalue_yaw -145.0 20.0)
            (`/Engine/EditorBlueprintResources/StandardMacros.DoOnce` false
              (:`Completed`
                (set `self.PuzzleSolved` true)
                (bind _returnvalue_4 (`GameplayStatics.GetActorOfClass` "/Game/Interactables/Item_Interactions/Brush_Interactables/PlaneCutOtherPart25_Blueprint.PlaneCutOtherPart25_Blueprint_C"))
                (`self.K2_DestroyActor` _returnvalue_4)
                (bind _returnvalue_5 (`GameplayStatics.GetActorOfClass` "/Game/Interactables/Item_Interactions/Brush_Interactables/Box25_Blueprint.Box25_Blueprint_C"))
                (`self.K2_DestroyActor` _returnvalue_5)
                (bind _returnvalue_6 (`GameplayStatics.GetActorOfClass` "/Game/Sounds/PlaneCutOtherPart26_Blueprint.PlaneCutOtherPart26_Blueprint_C"))
                (`self.K2_DestroyActor` _returnvalue_6)
                (`self.Done`)))))))))

(event `self.Box.OnComponentBeginOverlap`
  (params (OverlappedComponent :type "PrimitiveComponent Object Reference") (OtherActor :type "Actor Object Reference") (OtherComp :type "PrimitiveComponent Object Reference") (OtherBodyIndex :type Integer) (bFromSweep :type Boolean) (SweepResult :type "HitResult Structure (by ref)"))
  (set `self.ColissionP3` true))

(event `self.Box.OnComponentEndOverlap`
  (params (OverlappedComponent :type "PrimitiveComponent Object Reference") (OtherActor :type "Actor Object Reference") (OtherComp :type "PrimitiveComponent Object Reference") (OtherBodyIndex :type Integer))
  (set `self.ColissionP3` false))

(fn `UserConstructionScript`)