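; Checks the solution of location puzzle 6 and shows the thanks-for-playing screen once it is solved.
; Box overlap events set a flag for presence in the trigger, without filtering the overlapping actor.
; Until solved, Tick polls seven puzzle pieces through GetActorOfClass after a one-tick delay.
; Success requires that flag, a specific pattern of piece visibility flags and the archeologist facing a target yaw within a tolerance.
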(event `self.ReceiveTick`
  (params (DeltaSeconds :type "Float (single-precision)"))
  (if (not (`self.PuzzleSolved`))
    (`KismetSystemLibrary.DelayUntilNextTick`)
    (bind _returnvalue (`GameplayStatics.GetActorOfClass` "/Game/Interactables/Lever/PlaneCutOtherPart17_Blueprint.PlaneCutOtherPart17_Blueprint_C"))
    (set `self.Visibale1` (`/Game/Interactables/Lever/PlaneCutOtherPart17_Blueprint.visi` _returnvalue))
    (bind _returnvalue_2 (`GameplayStatics.GetActorOfClass` "/Game/Interactables/Lever/PlaneCutOtherPart18_Blueprint.PlaneCutOtherPart18_Blueprint_C"))
    (set `self.Visibale2` (`/Game/Interactables/Lever/PlaneCutOtherPart18_Blueprint.Visi` _returnvalue_2))
    (bind _returnvalue_3 (`GameplayStatics.GetActorOfClass` "/Game/Interactables/Lever/PlaneCutOtherPart19_Blueprint.PlaneCutOtherPart19_Blueprint_C"))
    (set `self.NewVar` (`/Game/Interactables/Lever/PlaneCutOtherPart19_Blueprint.Visi` _returnvalue_3))
    (bind _returnvalue_4 (`GameplayStatics.GetActorOfClass` "/Game/Interactables/Lever/PlaneCutOtherPart20_Blueprint.PlaneCutOtherPart20_Blueprint_C"))
    (set `self.NewVar_0` (`/Game/Interactables/Lever/PlaneCutOtherPart20_Blueprint.Visi` _returnvalue_4))
    (bind _returnvalue_5 (`GameplayStatics.GetActorOfClass` "/Game/Interactables/Lever/PlaneCutOtherPart14_Blueprint.PlaneCutOtherPart14_Blueprint_C"))
    (set `self.NewVar_2` (`/Game/Interactables/Lever/PlaneCutOtherPart14_Blueprint.Visi` _returnvalue_5))
    (bind _returnvalue_6 (`GameplayStatics.GetActorOfClass` "/Game/Interactables/Lever/Box14_Blueprint.Box14_Blueprint_C"))
    (set `self.NewVar_3` (`/Game/Interactables/Lever/Box14_Blueprint.Visi` _returnvalue_6))
    (bind _returnvalue_7 (`GameplayStatics.GetActorOfClass` "/Game/Interactables/Lever/PlaneCutOtherPart2_Blueprint.PlaneCutOtherPart2_Blueprint_C"))
    (set `self.NewVar_4` (`/Game/Interactables/Lever/PlaneCutOtherPart2_Blueprint.Visi` _returnvalue_7))
    (if (`self.ColissionP3`)
      (if (`self.Visibale1`)
        _
        (elif (`self.Visibale2`)
          _
          (elif (`self.NewVar`)
            _
            (elif (`self.NewVar_0`)
              _
              (elif (`self.NewVar_2`)
                (if (`self.NewVar_3`)
                  (if (`self.NewVar_4`)
                    (bind _returnvalue_8 (`GameplayStatics.GetActorOfClass` "/Game/Characters/HiddenPerspective/BP_Archeologist.BP_Archeologist_C"))
                    (bind (_returnvalue_roll _returnvalue_pitch _returnvalue_yaw) (`KismetMathLibrary.BreakRotator` (`self.K2_GetActorRotation` _returnvalue_8)))
                    (if (`KismetMathLibrary.NearlyEqual_FloatFloat` _returnvalue_yaw -60.0 20.0)
                      (set `self.PuzzleSolved` true)
                      (`/Engine/EditorBlueprintResources/StandardMacros.DoOnce` false
                        (:`Completed`
                          (bind _returnvalue_9 (`|CreateWidget` "/Game/UI/WB_ThanksForPlaying.WB_ThanksForPlaying_C"))
                          (`UserWidget.AddToViewport` _returnvalue_9 0))))))))))))))

(event `self.Box.OnComponentBeginOverlap`
  (params (OverlappedComponent :type "PrimitiveComponent Object Reference") (OtherActor :type "Actor Object Reference") (OtherComp :type "PrimitiveComponent Object Reference") (OtherBodyIndex :type Integer) (bFromSweep :type Boolean) (SweepResult :type "HitResult Structure (by ref)"))
  (set `self.ColissionP3` true))

(event `self.Box.OnComponentEndOverlap`
  (params (OverlappedComponent :type "PrimitiveComponent Object Reference") (OtherActor :type "Actor Object Reference") (OtherComp :type "PrimitiveComponent Object Reference") (OtherBodyIndex :type Integer))
  (set `self.ColissionP3` false))

(fn `UserConstructionScript`)