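; BP_Button3 is an interactable button that raises its cube when Button 2 is pressed and announces its own press.
; On BeginPlay it finds a BP_Button2 actor in the level and binds to its pressed event.
; That event plays the Appear timeline, which lerps the cube's relative Z upward.
; BeginInteraction runs the parent logic, then broadcasts Button3Pressed for any listeners.
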(event `self.ReceiveBeginPlay`
  (bind _returnvalue (`GameplayStatics.GetActorOfClass` "/Game/Interactables/Buttons/BP_Button2.BP_Button2_C"))
  (add `/Game/Interactables/Buttons/BP_Button2.Button2Pressed` _returnvalue (delegate `Button2Pressed`)))

(event `Button2Pressed`
  (bind (_direction _newtrack_0) (`Timeline|Appear`)
    (:`Update`
      (`SceneComponent.K2_SetRelativeLocation` (`self.Cube`) (`KismetMathLibrary.MakeVector` 0.0 0.0 (`KismetMathLibrary.Lerp` 50.0 150.0 _newtrack_0)) false false))))

(event `self.BeginInteraction`
  (`parent.BeginInteraction`)
  (`self.Button3Pressed`))

(fn `UserConstructionScript`
  (`parent.UserConstructionScript`))