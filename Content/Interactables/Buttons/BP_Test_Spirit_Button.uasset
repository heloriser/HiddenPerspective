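; BP_Test_Spirit_Button is a test interactable spirit button that signals its own press and reacts to another button.
; On BeginPlay it finds a BP_Button4 actor and binds to that actor's Button4Pressed dispatcher.
; When that fires, a Timeline lerps the relative Z location of its Cube to raise it.
; Interacting with it runs the parent logic, then broadcasts SpiritButton2Pressed.
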(event `self.ReceiveBeginPlay`
  (bind _returnvalue (`GameplayStatics.GetActorOfClass` "/Game/Interactables/Buttons/BP_Button4.BP_Button4_C"))
  (add `/Game/Interactables/Buttons/BP_Button4.Button4Pressed` _returnvalue (delegate `Button2Pressed`)))

(event `Button2Pressed`
  (bind (_direction _newtrack_0) (`Timeline|Timeline`)
    (:`Update`
      (`SceneComponent.K2_SetRelativeLocation` (`self.Cube`) (`KismetMathLibrary.MakeVector` 0.0 0.0 (`KismetMathLibrary.Lerp` 50.0 150.0 _newtrack_0)) false false))))

(event `self.BeginInteraction`
  (`parent.BeginInteraction`)
  (`self.SpiritButton2Pressed`))

(fn `UserConstructionScript`
  (`parent.UserConstructionScript`))