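; BP_Controller_Archaeologist handles Enhanced Input movement for the player-controlled archaeologist.
; BeginPlay adds the IMC_Actions and IMC_Looking mapping contexts to player 0's input subsystem at equal priority.
; The forward/back and left/right actions feed AddMovementInput along the actor's forward and right vectors.
; No look action is handled in this graph, and Tick and the construction script are empty.
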(event `self.ReceiveBeginPlay`
  (`EnhancedInputSubsystemInterface.AddMappingContext` (pcsubsystem `EnhancedInputLocalPlayerSubsystem` (`GameplayStatics.GetPlayerController` 0)) "/Game/Our_Stuff/Player_Controller/IMC_Actions.IMC_Actions" 0 (struct))
  (`EnhancedInputSubsystemInterface.AddMappingContext` (pcsubsystem `EnhancedInputLocalPlayerSubsystem` (`GameplayStatics.GetPlayerController` 0)) "/Game/Our_Stuff/Player_Controller/IMC_Looking.IMC_Looking" 0 (struct)))

(event `EnhancedInput|/Game/Our_Stuff/Player_Controller/IA_ForwardBack`
  (params (ActionValue :type "Float (double-precision)") (ElapsedSeconds :type "Float (double-precision)") (TriggeredSeconds :type "Float (double-precision)") (InputAction :type "InputAction Object Reference" :default "/Game/Our_Stuff/Player_Controller/IA_ForwardBack.IA_ForwardBack"))
  (:`Triggered`
    (`Pawn.AddMovementInput` (`self.GetActorForwardVector`) ActionValue)))

(event `EnhancedInput|/Game/Our_Stuff/Player_Controller/IA_LeftRight`
  (params (ActionValue :type "Float (double-precision)") (ElapsedSeconds :type "Float (double-precision)") (TriggeredSeconds :type "Float (double-precision)") (InputAction :type "InputAction Object Reference" :default "/Game/Our_Stuff/Player_Controller/IA_LeftRight.IA_LeftRight"))
  (:`Triggered`
    (`Pawn.AddMovementInput` (`self.GetActorRightVector`) ActionValue)))

(fn `UserConstructionScript`)